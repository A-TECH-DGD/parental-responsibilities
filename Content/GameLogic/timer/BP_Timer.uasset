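; BP_Timer is a countdown actor that shows a timer widget at BeginPlay and a lose widget when time runs out.
; Tick passes through a one-second Delay, so InitTimer drops by only one frame's DeltaSeconds about once per second.
; Nothing stops the countdown at zero, so the lose widget is created again on each later pass.
; BeginPlay also sets a non-looping timer by name on "Event Tick".
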(event EventTick
  (params (DeltaSeconds :type Float%20%28single-precision%29))
  (Utilities|FlowControl|Delay 1.0)
  (bind _output_get (Variables|Default|SetinitTimer (- (Variables|Default|GetinitTimer) DeltaSeconds)))
  (if (<= _output_get 0)
    (Development|PrintString "Time's Up!" false)
    (bind _returnvalue (UserInterface|CreateWidget "/Game/GameLogic/timer/WB_lose.WB_lose_C"))
    (UserInterface|Viewport|AddtoViewport _returnvalue 0)
    (else
      (Development|PrintString (Utilities|String|ToString(Integer) (Variables|Default|GetinitTimer)) false))))

(event EventBeginPlay
  (Utilities|Time|SetTimerbyFunctionName 0 "Event Tick" 1.0)
  (bind _returnvalue (UserInterface|CreateWidget "/Game/GameLogic/timer/WB_timer.WB_timer_C"))
  (UserInterface|Viewport|AddtoViewport _returnvalue 0))

(fn ConstructionScript)